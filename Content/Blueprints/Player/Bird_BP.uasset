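; Player bird for a Flappy Bird-style game: left click flaps, Tab toggles the HUD's difficulty, and any hit triggers death.
; Flaps zero capsule velocity before an upward impulse, while Tick pushes down as it rises, both using difficulty data.
; A save game persists high score and difficulty, restored once the HUD is set up.
; Death saves the record, disables flapping, then shows game-over scores after a delay.
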(event `self.ReceiveBeginPlay`
  (bind _savegame (`self.HandleSaveGameInitialization` (`self.saveGameName`)))
  (bind _ashud_base_setup (`/Game/Blueprints/Macros/BML_PlayerPawn.Get_HUD_BaseSetup` 10.0)
    (:`Success`
      (set `self.playerBaseHud` _ashud_base_setup)
      (bind _difficulty (`/Game/Blueprints/Save/HighScore_Save.difficulty` _savegame))
      (`/Engine/EditorBlueprintResources/StandardMacros.IsValid` _difficulty
        (:`Is Valid`
          (bind _output_get (set `self.difficultyData` _difficulty))
          (`self.SetDifficulty` _output_get))))))

(event `self.ReceiveTick`
  (params (DeltaSeconds :type "Float (single-precision)"))
  ;[1 1 1] Tick
  (`self.MoveDown`))

(event `Key|LeftMouseButton`
  (params (Key :type "Key Structure"))
  ;[1 0.8039 0.2999] Input
  (:`Pressed`
    (`GameplayStatics.PlaySoundAtLocation` "/Game/Assets/SFX/FlapSoundCue.FlapSoundCue" (`self.K2_GetActorLocation`) (struct) 1.0 1.0 0.0 null null null null)
    (`self.TryMoveUp`)))

(event `Key|Tab` :paused true
  (params (Key :type "Key Structure"))
  ;[1 0.8039 0.2999] Input
  (:`Pressed`
    (`/Game/Blueprints/Macros/HUD_BaseSetup.ToggleDifficulty` (`self.playerBaseHud`))))

(event `self.ReceiveHit`
  (params (MyComp :type "PrimitiveComponent Object Reference") (Other :type "Actor Object Reference") (OtherComp :type "PrimitiveComponent Object Reference") (bSelfMoved :type Boolean) (HitLocation :type "Vector Structure") (HitNormal :type "Vector Structure") (NormalImpulse :type "Vector Structure") (Hit :type "HitResult Structure (by ref)"))
  ;[1 1 1] Hit a wall
  (`self.Died`))

(event `Died`
  ;[1 1 1] Died
  (`self.SetHighScoreSave` (`self.score`))
  (`self.DieView`)
  (`KismetSystemLibrary.Delay` 0.5)
  (`self.BuildGameOverView`))

(event `AddScore`
  ;[1 1 1] Score
  (`GameplayStatics.PlaySoundAtLocation` "/Game/Assets/SFX/SFX_Score_01.SFX_Score_01" (`self.K2_GetActorLocation`) (struct) 1.0 1.0 0.0 null null null null)
  (`self.CalculateScore` (`self.scoreToAdd`)))

(fn `BuildGameOverView`
  ;[1 1 1] copies jr behavior. Linking widgets on player pawn
  (bind _returnvalue (`|CreateWidget` "/Game/Blueprints/Widgets/Gameplay/GameOver_WBP.GameOver_WBP_C"))
  (bind _output_get (set `self.gameOverHud` _returnvalue))
  (`/Game/Blueprints/Widgets/Gameplay/GameOver_WBP.SetScoreText` _output_get (`self.score`))
  (`/Game/Blueprints/Widgets/Gameplay/GameOver_WBP.SetHighScoreText` (`self.gameOverHud`) (`/Game/Blueprints/Save/HighScore_Save.highScore` (`self.HighScoreSaveRef`)))
  (`UserWidget.AddToViewport` (`self.gameOverHud`) 0))

(fn `CalculateScore`
  (params (factor :type Integer))
  (set `self.score` (+ (`self.score`) factor)))

(fn `DieView`
  (`/Engine/EditorBlueprintResources/StandardMacros.DoOnce` false
    (:`Completed`
      (`GameplayStatics.PlaySoundAtLocation` "/Game/Assets/SFX/SFX_HitObstacle_01.SFX_HitObstacle_01" (`self.K2_GetActorLocation`) (struct) 1.0 1.0 0.0 null null null null)
      (set `self.canMove` false)
      (`PrimitiveComponent.SetConstraintMode` (`self.Capsule`) "XZPlane"))))

(fn `HandleSaveGameInitialization`
  (params (SlotName :type String))
  (returns (saveGame :type "/Game/Blueprints/Save/HighScore_Save Object Reference"))
  (bind _returnvalue (`GameplayStatics.DoesSaveGameExist` SlotName))
  (if _returnvalue
    (bind _returnvalue_2 (`GameplayStatics.LoadGameFromSlot` (`self.saveGameName`)))
    (bind _ashigh_score_save (cast `/Game/Blueprints/Save/HighScore_Save` _returnvalue_2))
    (bind _output_get (set `self.HighScoreSaveRef` _ashigh_score_save))
    (return _output_get)
    (else
      (bind _returnvalue_3 (`GameplayStatics.CreateSaveGameObject` "/Game/Blueprints/Save/HighScore_Save.HighScore_Save_C"))
      (bind _output_get_2 (set `self.HighScoreSaveRef` _returnvalue_3))
      (`GameplayStatics.SaveGameToSlot` _output_get_2 (`self.saveGameName`)))))

(fn `MoveDown`
  (bind _returnvalue (`PrimitiveComponent.GetPhysicsLinearVelocity` (`self.Capsule`) "None"))
  (if (> (.z _returnvalue) 0.0)
    (`PrimitiveComponent.AddImpulse` (`self.Capsule`) (`/Game/DataAsset/DifficultyData/DifficultyAsset.GetImpulseDown` (`self.difficultyData`)) "None" false)))

(fn `SetDifficulty`
  (params (newData :type "/Game/DataAsset/DifficultyData/DifficultyAsset Object Reference"))
  (bind _highscoresaveref (`self.HighScoreSaveRef`))
  (bind _output_get (set `self.difficultyData` newData))
  (set `self.impulseUp` (`/Game/DataAsset/DifficultyData/DifficultyAsset.GetImpulseUp` _output_get))
  (set `self.impulseDown` (`/Game/DataAsset/DifficultyData/DifficultyAsset.GetImpulseDown` _output_get))
  (set `/Game/Blueprints/Save/HighScore_Save.difficulty` _output_get _highscoresaveref)
  (`GameplayStatics.SaveGameToSlot` _highscoresaveref (`self.saveGameName`)))

(fn `SetHighScoreSave`
  (params (A :type Integer))
  (bind _highscoresaveref (`self.HighScoreSaveRef`))
  (if (> A (`/Game/Blueprints/Save/HighScore_Save.highScore` (`self.HighScoreSaveRef`)))
    (set `/Game/Blueprints/Save/HighScore_Save.highScore` (`self.score`) _highscoresaveref)
    (`GameplayStatics.SaveGameToSlot` _highscoresaveref (`self.saveGameName`))))

(fn `SetMovementDown`
  (params (impulse :type "Vector Structure"))
  (set `self.impulseDown` impulse))

(fn `SetMovementUp`
  (params (impulse :type "Vector Structure"))
  (set `self.impulseUp` impulse))

(fn `TryMoveUp`
  (bind _capsule (`self.Capsule`))
  (if (`self.canMove`)
    (`PrimitiveComponent.SetPhysicsLinearVelocity` _capsule (0.0 0.0 0.0) false "None")
    (`PrimitiveComponent.AddImpulse` _capsule (`/Game/DataAsset/DifficultyData/DifficultyAsset.GetImpulseUp` (`self.difficultyData`)) "None" false)))

(fn `UserConstructionScript`)
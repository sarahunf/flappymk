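; Obstacle spawner actor that spawns obstacles continuously from the start of play.
; A delay macro loops back into the SpawnObstacle event, producing a new obstacle at a fixed short interval.
; Each spawn uses the spawner's transform, offset in Z by a random value within the difficulty Mode's min/max range.
; SetDifficulty stores that Mode reference after a validity check.
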(event `self.ReceiveBeginPlay`
  (`self.SpawnObstacle`))

(event `SpawnObstacle`
  (`self.SpawnObstacleWithDelay`))

(fn `SetDifficulty`
  (params (mode :type "/Game/DataAsset/DifficultyData/DifficultyAsset Object Reference"))
  (`/Engine/EditorBlueprintResources/StandardMacros.IsValid` mode
    (:`Is Valid`
      (set `self.mode` mode)
      (return))))

(fn `SpawnObstacleRandomZAxis`
  (bind (_returnvalue_location _returnvalue_rotation _returnvalue_scale) (`KismetMathLibrary.BreakTransform` (`self.GetTransform`)))
  (`|SpawnActorFromClass` "/Game/Blueprints/Obstacle/Obstacle_BP.Obstacle_BP_C" (`KismetMathLibrary.MakeTransform` (+ _returnvalue_location (`KismetMathLibrary.MakeVector` 0.0 0.0 (`KismetMathLibrary.RandomFloatInRange` (`/Game/DataAsset/DifficultyData/DifficultyAsset.GetObstaclesMinSpawnPosition` (`self.mode`)) (`/Game/DataAsset/DifficultyData/DifficultyAsset.GetObstaclesMaxSpawnPosition` (`self.mode`))))) _returnvalue_rotation _returnvalue_scale) "Undefined" "MultiplyWithRoot" null null))

(fn `UserConstructionScript`)
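; HUD Blueprint for a bird game that creates and manages the player HUD and game menu widgets.
; BeginPlay retries every two seconds until the pawn casts to Bird_BP, then adds both the player HUD and difficulty menu to the viewport.
; ToggleWidget collapses other listed menus and switches the target between paused, cursor-enabled UI and gameplay.
; Difficulty changes toggle the menu and update the HUD's stars; game-over setup is unconnected.
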(event `self.ReceiveBeginPlay`
  (bind _gamemenuwidgetlist (`self.gameMenuWidgetList`))
  ;[1 0 0] This could keep leaking forever if class was not that obvious
  (bind _asbird_bp (cast `/Game/Blueprints/Player/Bird_BP` (`GameplayStatics.GetPlayerPawn` 0) :!label _label)
    (:`then`
      (set `self.player` _asbird_bp)
      ;[1 1 1] Game
      (bind _returnvalue (`|CreateWidget` "/Game/Blueprints/Widgets/Gameplay/PlayerHUD_WBP.PlayerHUD_WBP_C" null (`self.player`)))
      (bind _output_get (set `self.playerHud` _returnvalue))
      (`UserWidget.AddToViewport` _output_get 0)
      ;[1 1 1] Game Menu's
      (bind _returnvalue_2 (`|CreateWidget` "/Game/Blueprints/Widgets/Gameplay/Difficulty_WBP.Difficulty_WBP_C"))
      (bind _output_get_2 (set `self.difficultyHud` _returnvalue_2))
      (`KismetArrayLibrary.Array_Add` _gamemenuwidgetlist _output_get_2)
      (for _array_element _gamemenuwidgetlist
        (`UserWidget.AddToViewport` _array_element 0)))
    (:`CastFailed`
      (`KismetSystemLibrary.Delay` 2.0)
      (goto _label))))

(event `ToggleDifficulty`
  (bind _difficultyhud (`self.difficultyHud`))
  ;[1 1 1] Difficulty
  (`self.ToggleWidget` _difficultyhud)
  (add `/Game/Blueprints/Widgets/Gameplay/Difficulty_WBP.DifficultyChanged` _difficultyhud (delegate `DifficultyChanged_Event`)))

(event `DifficultyChanged_Event`
  (params (mode :type "/Game/DataAsset/DifficultyData/DifficultyAsset Object Reference"))
  ;[1 1 1] Difficulty
  (`self.ToggleWidget` (`self.difficultyHud`))
  (`/Game/Blueprints/Widgets/Gameplay/PlayerHUD_WBP.UpdateDifficultyStars` (`self.playerHud`) (`/Game/DataAsset/DifficultyData/DifficultyAsset.mode` mode)))

(fn `FocusGame`
  (bind _returnvalue (`self.GetOwningPlayerController`))
  (`Widget.SetVisibility` (`self.focusedWidget`) "Collapsed")
  (`WidgetBlueprintLibrary.SetInputMode_GameOnly` _returnvalue)
  (set `PlayerController.bShowMouseCursor` false _returnvalue)
  (`GameplayStatics.SetGamePaused` false))

(fn `FocusWidget`
  (bind _returnvalue (`self.GetOwningPlayerController`))
  (`Widget.SetVisibility` (`self.focusedWidget`) "SelfHitTestInvisible")
  (`WidgetBlueprintLibrary.SetInputMode_GameAndUIEx` _returnvalue (`self.focusedWidget`))
  (set `PlayerController.bShowMouseCursor` true _returnvalue)
  (`GameplayStatics.SetGamePaused` true))

(fn `ToggleWidget`
  (params (targetWidget :type "UserWidget Object Reference"))
  (`/Engine/EditorBlueprintResources/StandardMacros.IsValid` targetWidget
    (:`Is Valid`
      (set `self.focusedWidget` targetWidget)
      (for _array_element (`self.gameMenuWidgetList`)
        (`/Engine/EditorBlueprintResources/StandardMacros.IsValid` _array_element
          (:`Is Valid`
            (if (== (`self.focusedWidget`) _array_element)
              (if (`Widget.IsVisible` (`self.focusedWidget`))
                (`self.FocusGame`)
                (else
                  (`self.FocusWidget`)))
              (elif (`Widget.IsVisible` _array_element)
                (`Widget.SetVisibility` _array_element "Collapsed")))))))))

(fn `UserConstructionScript`)